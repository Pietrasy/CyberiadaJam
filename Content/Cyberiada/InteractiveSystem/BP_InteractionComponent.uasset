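; Actor component that lets its owning Character interact with nearby actors implementing BPI_Interactable.
; It caches the owner on BeginPlay and binds to the capsule's begin and end overlap events to maintain a list of interactables in range.
; The IA_Interact input sends an interact message to the first listed actor, passing player character 0 rather than the cached owner.
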(event `self.ReceiveBeginPlay`
  (`self.CacheOwner`)
  (add `PrimitiveComponent.OnComponentBeginOverlap` (`Character.CapsuleComponent` (`self.Owner`)) (`|CreateDelegate` :!event `HandleCapsuleOverlapBegin`))
  (add `PrimitiveComponent.OnComponentEndOverlap` (`Character.CapsuleComponent` (`self.Owner`)) (`|CreateDelegate` :!event `HandleCapsuleOverlapEnd`)))

(event `HandleCapsuleOverlapBegin`
  (params (OverlappedComponent :type "PrimitiveComponent Object Reference") (OtherActor :type "Actor Object Reference") (OtherComp :type "PrimitiveComponent Object Reference") (OtherBodyIndex :type Integer) (bFromSweep :type Boolean) (SweepResult :type "HitResult Structure (by ref)"))
  (if (`KismetSystemLibrary.DoesImplementInterface` OtherActor "/Game/Cyberiada/InteractiveSystem/BPI_Interactable.BPI_Interactable_C")
    (`KismetArrayLibrary.Array_AddUnique` (`self.InteractablesInRange`) OtherActor)))

(event `HandleCapsuleOverlapEnd`
  (params (OverlappedComponent :type "PrimitiveComponent Object Reference") (OtherActor :type "Actor Object Reference") (OtherComp :type "PrimitiveComponent Object Reference") (OtherBodyIndex :type Integer))
  (if (`KismetSystemLibrary.DoesImplementInterface` OtherActor "/Game/Cyberiada/InteractiveSystem/BPI_Interactable.BPI_Interactable_C")
    (`KismetArrayLibrary.Array_RemoveItem` (`self.InteractablesInRange`) OtherActor)))

(event `EnhancedInput|/Game/Cyberiada/InteractiveSystem/IA_Interact`
  (params (ActionValue :type Boolean) (ElapsedSeconds :type "Float (double-precision)") (TriggeredSeconds :type "Float (double-precision)") (InputAction :type "InputAction Object Reference" :default "/Game/Cyberiada/InteractiveSystem/IA_Interact.IA_Interact"))
  (:`Started`
    (if (`KismetArrayLibrary.Array_IsNotEmpty` (`self.InteractablesInRange`))
      (`self.InteractWithActor` (`|GetArrayItem` (`self.InteractablesInRange`))))))

(fn `CacheOwner`
  (bind _ascharacter (cast `Character` (`self.GetOwner`)))
  (set `self.Owner` _ascharacter)
  (return))

(fn `InteractWithActor`
  (params (InActor :type "Actor Object Reference"))
  (`/Engine/EditorBlueprintResources/StandardMacros.IsValid` InActor
    (:`Is Valid`
      (message `/Game/Cyberiada/InteractiveSystem/BPI_Interactable.Interact` (`local.InActor`) (`GameplayStatics.GetPlayerCharacter` 0))
      (return))
    (:`Is Not Valid`
      (return))))