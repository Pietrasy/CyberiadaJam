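; BP_AnomalyManager is a manager that triggers the BP_Anomaly actors placed in the level.
; On BeginPlay it caches every BP_Anomaly, then offers activation of all of them (the level input is unused) or of one at random.
; The random pick calls itself recursively past invalid or disabled entries, with no exit if none qualifies.
; A separate function schedules that random pick on a timer, but nothing here calls it.
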(event `self.ReceiveBeginPlay`
  (`self.CacheAnomalies`))

(fn `ActivateAnomalies`
  (params (InAnomalyLevel :type Integer))
  (locals (AnomalyFromArray :type "/Game/Cyberiada/Blueprints/Anomalies/BP_Anomaly Object Reference"))
  (for _array_element (`self.Anomalies`)
    (`/Game/Cyberiada/Blueprints/Anomalies/BP_Anomaly.ActivateAnomaly` _array_element))
  (return))

(fn `ActiveRandomAnomaly`
  (locals (AnomalyFromArray :type "/Game/Cyberiada/Blueprints/Anomalies/BP_Anomaly Object Reference"))
  (if (`KismetArrayLibrary.Array_IsNotEmpty` (`self.Anomalies`))
    (bind _output_get (set `local.AnomalyFromArray` (`KismetArrayLibrary.Array_Random` (`self.Anomalies`))))
    (`/Engine/EditorBlueprintResources/StandardMacros.IsValid` _output_get
      (:`Is Valid`
        (if (`/Game/Cyberiada/Blueprints/Anomalies/BP_Anomaly.GetIsDisable` (`local.AnomalyFromArray`))
          (`self.ActiveRandomAnomaly`)
          (return)
          (else
            (`/Game/Cyberiada/Blueprints/Anomalies/BP_Anomaly.ActivateAnomaly` (`local.AnomalyFromArray`))
            (return))))
      (:`Is Not Valid`
        (`self.ActiveRandomAnomaly`)
        (return)))
    (else
      (`KismetSystemLibrary.PrintString` "Array with anomalies is empty!")
      (return))))

(fn `CacheAnomalies`
  (bind _outactors (`GameplayStatics.GetAllActorsOfClass` "/Game/Cyberiada/Blueprints/Anomalies/BP_Anomaly.BP_Anomaly_C"))
  (set `self.Anomalies` _outactors)
  (return))

(fn `SetTimerForNextAnomaly`
  (bind _returnvalue (`KismetSystemLibrary.K2_SetTimer` null "ActiveRandomAnomaly" (`self.TimeToAnomaly`)))
  (set `self.ActiveRandomAnomaly_TimerHandle` _returnvalue)
  (return))

(fn `UserConstructionScript`)