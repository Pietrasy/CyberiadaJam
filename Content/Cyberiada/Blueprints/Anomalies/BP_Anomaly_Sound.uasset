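; BP_Anomaly_Sound is an anomaly that plays a sound at its location while active until the player fixes it.
; Activation calls the parent logic, spawns the sound, stores the audio component and binds its finished event, apparently to a custom event that replays it as a manual loop.
; Interacting fixes the anomaly, destroying the audio component, and then fires the OnInteract call.
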(event `CustomEvent`
  (bind _soundinstance (`self.SoundInstance`)
    (:`then`
      (`AudioComponent.Play` _soundinstance 0.0))
    (:`else`)))

(event `/Game/Cyberiada/InteractiveSystem/BPI_Interactable.Interact`
  (params (Interactor :type "Actor Object Reference"))
  (`self.FixAnomaly`)
  (`self.OnInteract`))

(fn `ActivateAnomaly`
  (`parent.ActivateAnomaly`)
  (bind _returnvalue (`GameplayStatics.SpawnSoundAtLocation` (`self.Sound_0`) (`self.K2_GetActorLocation`) (struct) 1.0 1.0 0.0 null null false))
  (bind _output_get (set `self.SoundInstance` _returnvalue))
  (add `AudioComponent.OnAudioFinished` _output_get (`|CreateDelegate` :!event `CustomEvent`)))

(fn `FixAnomaly`
  (`parent.FixAnomaly`)
  (bind _soundinstance (`self.SoundInstance`)
    (:`then`
      (`ActorComponent.K2_DestroyComponent` _soundinstance))
    (:`else`)))

(fn `UserConstructionScript`
  (`parent.UserConstructionScript`))