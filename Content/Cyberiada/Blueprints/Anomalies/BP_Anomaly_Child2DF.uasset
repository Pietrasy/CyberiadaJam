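; Child anomaly actor that turns to face the first player's character.
; Every Tick, it computes a look-at rotation toward that character and applies it through RInterpTo with no interp speed set, so it snaps rather than eases.
; The construction script only calls the parent's.
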(event `self.ReceiveTick`
  (params (DeltaSeconds :type "Float (single-precision)"))
  (`self.K2_SetActorRotation` (`KismetMathLibrary.RInterpTo` (`self.K2_GetActorRotation` self) (`KismetMathLibrary.FindLookAtRotation` (`self.K2_GetActorLocation` self) (`self.K2_GetActorLocation` (`GameplayStatics.GetPlayerCharacter` 0))) DeltaSeconds)))

(fn `UserConstructionScript`
  (`parent.UserConstructionScript`))