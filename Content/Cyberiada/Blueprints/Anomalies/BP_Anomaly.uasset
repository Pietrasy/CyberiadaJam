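; BP_Anomaly is an anomaly actor for a horror game that can be activated, fixed, disabled and enabled.
; Activating or fixing it sets state flags, raises or lowers insanity through BP_HorrorGameMode, then fires a matching event dispatcher.
; Interacting only broadcasts an OnInteract dispatcher, and the Construction Script applies the configurable AnomalyMesh to the static mesh component.
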(event `/Game/Cyberiada/InteractiveSystem/BPI_Interactable.Interact`
  (params (Interactor :type "Actor Object Reference"))
  (`self.OnInteract`))

(fn `ActivateAnomaly`
  (set `self.IsActive` true)
  (bind _asbp_horror_game_mode (cast `/Game/Variant_Horror/Blueprints/BP_HorrorGameMode` (`GameplayStatics.GetGameMode`)))
  (`/Game/Variant_Horror/Blueprints/BP_HorrorGameMode.IncreaseInsanity` _asbp_horror_game_mode)
  (`self.OnActivateAnomaly`)
  (return))

(fn `DisableAnomaly`
  (set `self.IsDisable` true)
  (return))

(fn `EnableAnomaly`
  (set `self.IsDisable` false)
  (return))

(fn `FixAnomaly`
  (set `self.IsFix` true)
  (bind _asbp_horror_game_mode (cast `/Game/Variant_Horror/Blueprints/BP_HorrorGameMode` (`GameplayStatics.GetGameMode`)))
  (`/Game/Variant_Horror/Blueprints/BP_HorrorGameMode.DecreaseInsanity` _asbp_horror_game_mode)
  (`self.OnFixAnomaly`)
  (return))

(fn `GetIsDisable`
  (returns (IsDisable :type Boolean))
  (return (`self.IsDisable`)))

(fn `SetStaticMesh`
  (`StaticMeshComponent.SetStaticMesh` (`self.AnomalyStaticMesh`) (`self.AnomalyMesh`))
  (return))

(fn `UserConstructionScript`
  (`self.SetStaticMesh`))