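; BP_AnomalyManager keeps track of the BP_Anomaly actors in the world and activates them on demand.
; CacheAnomalies fills the Anomalies array with GetAllActorsOfClass, and both activation functions read from that cached list.
; ActivateAnomalies triggers every anomaly matching a given AnomalyLevel, while ActiveRandomAnomaly triggers one random pick regardless of level.
; It has no event graph logic, so caching and activation depend on outside calls.
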(fn `ActivateAnomalies`
  (params (InAnomalyLevel :type Integer))
  (locals (AnomalyFromArray :type "/Game/Cyberiada/Blueprints/Anomalies/BP_Anomaly Object Reference"))
  (for _array_element (`self.Anomalies`)
    (bind _output_get (set `local.AnomalyFromArray` _array_element))
    (if (== (`/Game/Cyberiada/Blueprints/Anomalies/BP_Anomaly.AnomalyLevel` _output_get) (`local.InAnomalyLevel`))
      (`/Game/Cyberiada/Blueprints/Anomalies/BP_Anomaly.ActivateAnomaly` (`local.AnomalyFromArray`))))
  (return))

(fn `ActiveRandomAnomaly`
  (`/Game/Cyberiada/Blueprints/Anomalies/BP_Anomaly.ActivateAnomaly` (`KismetArrayLibrary.Array_Random` (`self.Anomalies`)))
  (return))

(fn `CacheAnomalies`
  (bind _outactors (`GameplayStatics.GetAllActorsOfClass` "/Game/Cyberiada/Blueprints/Anomalies/BP_Anomaly.BP_Anomaly_C"))
  (set `self.Anomalies` _outactors))

(fn `UserConstructionScript`)