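; BP_Crewman is a flipbook character, shown for its matching room, that disappears after the player keeps looking at it.
; Entering its sphere starts a looping dot-product check of whether the camera faces it.
; Looking adds a shaking vignette post-process material and enables Tick, which fades the shake until the crewman broadcasts its disabling and destroys itself.
; Looking away resets the fade, removes the vignette and restarts a separate timer.
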(event `OnLookAt`
  (`/Engine/EditorBlueprintResources/StandardMacros.DoOnce` false :!label _label
    (:`Completed`
      (`MaterialInstanceDynamic.SetScalarParameterValue` (`self.Vignette`) "Shake Intensity" 0.1)
      (`MaterialInstanceDynamic.SetScalarParameterValue` (`self.Vignette`) "Horizontal Movement" 0.9)
      (`MaterialInstanceDynamic.SetScalarParameterValue` (`self.Vignette`) "Vertical Movement" 0.9))))

(event `OnReset`
  (goto _label :!via `Reset`))

(event `self.Sphere.OnComponentBeginOverlap`
  (params (OverlappedComponent :type "PrimitiveComponent Object Reference") (OtherActor :type "Actor Object Reference") (OtherComp :type "PrimitiveComponent Object Reference") (OtherBodyIndex :type Integer) (bFromSweep :type Boolean) (SweepResult :type "HitResult Structure (by ref)"))
  (bind _returnvalue (`KismetSystemLibrary.K2_SetTimer` null "CheckIfPlayerIsLooking" 0.1 true true))
  (set `self.CheckIfPlayerIsLooking_TimerHandle` _returnvalue))

(event `SpawnCharacter`
  (params (InRoom :type "/Game/Cyberiada/Data/E_Room Enum" :default "NewEnumerator0"))
  (if (`|EnumEquality` (`self.Room`) InRoom)
    (`PaperFlipbookComponent.SetFlipbook` (`self.PaperFlipbook`) (`self.FlipBook`))))

(event `self.ReceiveTick`
  (params (DeltaSeconds :type "Float (single-precision)"))
  (bind _output_get (set `self.CurrentScale` (`KismetMathLibrary.Lerp` (`self.CurrentScale`) 0.0 (* (`GameplayStatics.GetWorldDeltaSeconds`) 1.0))))
  (bind _returnvalue (* _output_get 0.1))
  (`MaterialInstanceDynamic.SetScalarParameterValue` (`self.Vignette`) "Shake Intensity" _returnvalue)
  (`KismetSystemLibrary.PrintString` (`KismetStringLibrary.Conv_DoubleToString` _returnvalue))
  (if (<= _returnvalue 0.003)
    (`self.OnDisableCrewman`)
    (`self.K2_DestroyActor`)))

(event `DisableCrewman`
  (bind _asbp_first_person_character (cast `/Game/FirstPerson/Blueprints/BP_FirstPersonCharacter` (`GameplayStatics.GetPlayerCharacter` 0)))
  (`CameraComponent.RemoveBlendable` (`/Game/FirstPerson/Blueprints/BP_FirstPersonCharacter.FirstPersonCamera` _asbp_first_person_character) (`self.Vignette`))
  (`KismetSystemLibrary.K2_ClearAndInvalidateTimerHandle` (`self.TimerForVignette_TimerHandle`)))

(fn `AddVignette`
  (bind _returnvalue (`KismetMaterialLibrary.CreateDynamicMaterialInstance` "/Game/Art/Vignette/MI_Vignette_Shake.MI_Vignette_Shake"))
  (set `self.Vignette` _returnvalue)
  (bind _asbp_first_person_character (cast `/Game/FirstPerson/Blueprints/BP_FirstPersonCharacter` (`GameplayStatics.GetPlayerCharacter` 0)))
  (`CameraComponent.AddOrUpdateBlendable` (`/Game/FirstPerson/Blueprints/BP_FirstPersonCharacter.FirstPersonCamera` _asbp_first_person_character) (`self.Vignette`) 1.0))

(fn `CheckIfPlayerIsLooking`
  (bind _returnvalue (`GameplayStatics.GetPlayerCameraManager` 0))
  (if (< (`self.Angle`) (`KismetMathLibrary.Dot_VectorVector` (`self.GetActorForwardVector` _returnvalue) (`KismetMathLibrary.GetDirectionUnitVector` (`PlayerCameraManager.GetCameraLocation` _returnvalue) (`self.K2_GetActorLocation`))))
    (`self.AddVignette`)
    (`self.OnLookAt`)
    (`self.SetActorTickEnabled` true)
    (else
      (`self.ResetVignette`)
      (`self.ResetTimer`)
      (`self.OnReset`)
      (`self.SetActorTickEnabled` false))))

(fn `ResetTimer`
  (`KismetSystemLibrary.K2_ClearAndInvalidateTimerHandle` (`self.TimerForVignette_TimerHandle`))
  (`self.SetTimerForVignette`))

(fn `ResetVignette`
  (`MaterialInstanceDynamic.SetScalarParameterValue` (`self.Vignette`) "Shake Intensity" 1.0)
  (`MaterialInstanceDynamic.SetScalarParameterValue` (`self.Vignette`) "Horizontal Movement" 0.9)
  (`MaterialInstanceDynamic.SetScalarParameterValue` (`self.Vignette`) "Vertical Movement" 0.9)
  (set `self.CurrentScale` 1.0)
  (`self.DisableCrewman`))

(fn `SetTimerForVignette`
  (bind _returnvalue (`KismetSystemLibrary.K2_SetTimerDelegate` (`|CreateDelegate` :!event `DisableCrewman`) (`self.RequirementTime`)))
  (set `self.TimerForVignette_TimerHandle` _returnvalue))

(fn `UserConstructionScript`)