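; BP_ControlSystem drives a control system's lighting response to low energy and to anomalies.
; EnableLowEnergySystem cuts the intensity of every referenced light to a third of its current value, with no restore function.
; ToggleLamps switches off three control lamps progressively as the anomaly number crosses rising thresholds.
; Its nested checks re-enable only the first lamp below its threshold, leaving later lamps untouched.
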(fn `EnableLowEnergySystem`
  (for _array_element (`self.Lights`)
    (bind _lightcomponent (`Light.LightComponent` _array_element))
    (`LightComponent.SetIntensity` _lightcomponent (`KismetMathLibrary.SafeDivide` (`LightComponentBase.Intensity` _lightcomponent) 3.0))))

(fn `ToggleLamps`
  (params (InAnomalyNumber :type Integer))
  (bind _output (`|GetArrayItem` (`self.ControlLamps`)))
  (bind _output_2 (`|GetArrayItem` (`self.ControlLamps`) 1))
  (bind _output_3 (`|GetArrayItem` (`self.ControlLamps`) 2))
  (if (>= InAnomalyNumber 1)
    (`/Game/Cyberiada/Blueprints/ControlSystem/BP_ControlLamp.DisableLamp` _output)
    (if (>= (`local.InAnomalyNumber`) 2)
      (`/Game/Cyberiada/Blueprints/ControlSystem/BP_ControlLamp.DisableLamp` _output_2)
      (if (>= (`local.InAnomalyNumber`) 4)
        (`/Game/Cyberiada/Blueprints/ControlSystem/BP_ControlLamp.DisableLamp` _output_3)
        (else
          (`/Game/Cyberiada/Blueprints/ControlSystem/BP_ControlLamp.EnableLamp` _output_3)))
      (else
        (`/Game/Cyberiada/Blueprints/ControlSystem/BP_ControlLamp.EnableLamp` _output_2)))
    (else
      (`/Game/Cyberiada/Blueprints/ControlSystem/BP_ControlLamp.EnableLamp` _output))))

(fn `UserConstructionScript`)