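; BP_Spawner is a character actor that displays a Paper2D flipbook and turns to face the player.
; SpawnCharacter assigns the flipbook when the given room matches its Room variable; it spawns no new actor.
; BeginPlay passes its own Room, so the flipbook is set at start.
; Tick applies RInterpTo toward the look-at rotation to player 0, rotating the whole actor like a billboard without restricting it to yaw.
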(event `self.ReceiveBeginPlay`
  (`self.SpawnCharacter` (`self.Room`)))

(event `SpawnCharacter`
  (params (InRoom :type "/Game/Cyberiada/Blueprints/Characters/E_Room Enum" :default "NewEnumerator0"))
  (if (`|EnumEquality` (`self.Room`) InRoom)
    (`PaperFlipbookComponent.SetFlipbook` (`self.PaperFlipbook`) (`self.FlipBook`))))

(event `self.ReceiveTick`
  (params (DeltaSeconds :type "Float (single-precision)"))
  (`self.K2_SetActorRotation` (`KismetMathLibrary.RInterpTo` (`self.K2_GetActorRotation` self) (`KismetMathLibrary.FindLookAtRotation` (`self.K2_GetActorLocation` self) (`self.K2_GetActorLocation` (`GameplayStatics.GetPlayerCharacter` 0))) DeltaSeconds)))

(fn `UserConstructionScript`)